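; Health component that tracks its owner's health and infection, sending the owner a death message when health empties or infection maxes out.
; HeathBarWidgetRef fetches the HUD health bar through the owner's player message and initializes both bars.
; Infection rises in fixed steps, shrinking max health and updating the bar by ratio.
; Damage on a BP_Player owner sets the health bar to zero, leaving the computed health ratio unconnected.
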(event Custom|TakeDamage
  (params (Damage :type Float%20%28double-precision%29))
  (if (<= (- (Variables|Default|GetCurrentHeath) Damage) 0.0)
    (Variables|Default|SetCurrentHeath 0.0)
    (Class|BPIHelperHeathComponent|OnDeath(Message) (Components|GetOwner))
    (else
      (bind _output_get (Variables|Default|SetCurrentHeath (- (Variables|Default|GetCurrentHeath) Damage)))))
  (if (.bSuccess (Utilities|Casting|CastToBP_Player (Components|GetOwner)))
    (Default|SetHeath (Variables|Default|GetHeathWidgetRef) 0.0)))

(event Custom|TakeInfection
  (if (>= (+ (Variables|Default|GetCurrentInfection) 1e+01) (Variables|Default|GetMaxInfection))
    (Variables|Default|SetCurrentInfection (Variables|Default|GetMaxInfection))
    (Default|SetInfection (Variables|Default|GetHeathWidgetRef) 1.0)
    (Class|BPIHelperHeathComponent|OnDeath(Message) (Components|GetOwner))
    (else
      (bind _output_get (Variables|Default|SetCurrentInfection (+ (Variables|Default|GetCurrentInfection) 1e+01)))
      (Variables|Default|SetMaxHeath (- (Variables|Default|GetMaxHeath) 1e+01))
      (Default|SetInfection (Variables|Default|GetHeathWidgetRef) (/ _output_get (Variables|Default|GetMaxInfection))))))

(event EventBeginPlay
  (Variables|Default|SetCurrentHeath (Variables|Default|GetMaxHeath))
  (Variables|Default|SetCurrentInfection 0.0))

(event EventHeathBarWidgetRef
  (bind _playr (Class|BPIHelperHeathComponent|RefPlayr(Message) (Components|GetOwner)))
  (Variables|Default|SetHeathWidgetRef (Variables|/Game/UI/BP_PlayrHUD.BP_PlayrHUD_C|GetHeathBarWidgetRef (Variables|/Game/Blueprints/Player/BP_Player.BP_Player_C|GetPlayrHUDRef _playr)))
  (Default|SetHeath (Variables|Default|GetHeathWidgetRef) 1.0)
  (Default|SetInfection (Variables|Default|GetHeathWidgetRef) 0.0))

(fn RefPlayr
  (return 0))