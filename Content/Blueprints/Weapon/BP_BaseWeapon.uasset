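; Base weapon for BP_Player that handles hitscan firing, ammo, reloading and its HUD widget.
; WeaponFire plays montages, spends ammo, spawns a Niagara tracer and damages BP_BaseZombi with critical headshots, looping after FireRate for one WeaponType.
; The spread trace starts at the camera and is redone from the muzzle when the aim point lies behind it.
; WeaponReload refills the magazine from reserve ammo and re-enables firing when the montage completes.
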(event Custom|WeaponFire
  (bind _hitresuit (Variables|Default|GetHitResuit))
  (if (not (Variables|/Game/Blueprints/Player/BP_Player.BP_Player_C|GetIsStopFire (Variables|Default|GetPlayerRef))) :!label _label
    (Variables|FireWeapon|SetCanFire false)
    (Animation|Montage|PlayMontage (Variables|/Script/Engine.Character|GetMesh (Variables|Default|GetPlayerRef)) (Variables|AnimMontage|GetFireAnim)
      (:then
        (Animation|Montage|PlayMontage (Variables|Default|GetWeaponMesh) (Variables|AnimMontage|GetFireWeaponAnim)
          (:then
            (CallFunction|UpdateAmmoMagazin)
            (Default|UpdateAmmoInfo (Variables|UI|GetWeaponWidgetRef) (Class|KismetMathLibrary|ToInt64(Integer) (Variables|Ammo|GetAmmoMagazin)) (Class|KismetMathLibrary|ToInt64(Integer) (Variables|Ammo|GetCurrentAmmo)))
            (bind _hitresuit_2 (CallFunction|LineTraceLogic))
            (CallFunction|TraceEndPoint _hitresuit_2)
            (CallFunction|TraceFX)
            (bind _asbp_base_zombi (Utilities|Casting|CastToBP_BaseZombi (.hitactor _hitresuit))
              (:then
                (Game|Damage|ApplyDamage _asbp_base_zombi (Math|Float|SelectFloat (Variables|Default|GetCriticalDamage) (Variables|Default|GetDamage) (== (.hitbonename _hitresuit) "head")) 0 self))
              (:CastFailed
                _))
            (Utilities|FlowControl|Delay (Variables|FireWeapon|GetFireRate))
            (if (Variables|Default|GetMagazinEmpty)
              (Variables|FireWeapon|SetCanFire false)
              (Development|PrintString "Патроны закончились")
              (else
                (Variables|FireWeapon|SetCanFire true)
                (if (Utilities|Enum|Equal(Enum) (Variables|Default|GetWeaponType) "NewEnumerator1")
                  (goto _label))))))))))

(event Custom|WeaponReload
  (if (and (CallFunction|AmmoNotEmpty) (not (CallFunction|MagazinFull)))
    (Variables|Default|SetIsReload false)
    (CallFunction|CalculateAmmo)
    (Variables|Default|SetMagazinEmpty false)
    (Default|UpdateAmmoInfo (Variables|UI|GetWeaponWidgetRef) (Class|KismetMathLibrary|ToInt64(Integer) (Variables|Ammo|GetAmmoMagazin)) (Class|KismetMathLibrary|ToInt64(Integer) (Variables|Ammo|GetCurrentAmmo)))
    (Animation|Montage|PlayMontage (Variables|/Script/Engine.Character|GetMesh (Variables|Default|GetPlayerRef)) (Variables|AnimMontage|GetReloadAnim)
      (:OnCompleted
        (Variables|Default|SetIsReload false)
        (Variables|FireWeapon|SetCanFire true)))))

(event EventBeginPlay
  (bind _asbp_player (Utilities|Casting|CastToBP_Player (Components|GetOwner)))
  (Variables|Default|SetPlayerRef _asbp_player))

(fn ConstructionScript)

(fn AttachtoHand
  (params (HandSocket :type Name))
  (Transformation|AttachComponentToComponent (Variables|/Script/Engine.Character|GetMesh (Variables|Default|GetPlayerRef)) HandSocket "SnapToTarget" "SnapToTarget" "SnapToTarget" true))

(fn SetWeaponWidgetRef
  (params (WeaponWidget :type WBP%20Weapon%20Object%20Reference))
  (Variables|UI|SetWeaponWidgetRef WeaponWidget))

(fn UpdateWidgetInfo
  (Default|UpdateWeaponWidgetInfo (Variables|UI|GetWeaponWidgetRef) (Variables|Ammo|GetAmmoMagazin) (Variables|Ammo|GetCurrentAmmo) (Variables|UI|GetImageHud)))

(fn UpdateAmmoMagazin
  (bind _result (Math|Integer|DecrementInt (Variables|Ammo|GetAmmoMagazin))
    (:%20%20
      (if (== _result 0)
        (Variables|Default|SetMagazinEmpty true)))))

(fn LineTraceLogic
  (bind _returnvalue (Game|GetPlayerController 0))
  (bind _weaponmesh (Variables|Default|GetWeaponMesh))
  (bind _returnvalue_2 (Transformation|GetSocketLocation _weaponmesh "MuzzleFlash"))
  (bind (_location _rotation) (Pawn|GetPlayerViewPoint _returnvalue))
  (bind (_outhit _returnvalue_3) (Collision|LineTraceByChannel _location (Math|Random|RandomPointinBoundingBox (+ _location (* (Math|Rotator|GetRotationXVector _rotation) (Variables|FireWeapon|GetFireDistance))) (* "1.000000,1.000000,1.000000" (Variables|FireWeapon|GetSpread))) "TraceTypeQuery1" false 0 "None"))
  (if _returnvalue_3
    _
    (else
      _))
  (Variables|Default|SetHitResuit _outhit)
  (if (> (Class|KismetMathLibrary|DegAcos (Math|Vector|DotProduct (Math|Vector|GetForwardVector (Transformation|GetSocketRotation (Variables|Default|GetWeaponMesh) "MuzzleFlash")) (- (Math|Vector|SelectVector (.ImpactPoint (Collision|BreakHitResult _outhit)) (.TraceEnd (Collision|BreakHitResult _outhit)) (.bBlockingHit (Collision|BreakHitResult _outhit))) (Transformation|GetSocketLocation (Variables|Default|GetWeaponMesh) "MuzzleFlash")))) 9e+01)
    (bind _outhit_2 (Collision|LineTraceByChannel _returnvalue_2 (Math|Random|RandomPointinBoundingBox (+ _returnvalue_2 (* (Math|Vector|GetForwardVector (Transformation|GetSocketRotation (Variables|Default|GetWeaponMesh) "MuzzleFlash")) (Variables|FireWeapon|GetFireDistance))) (* "1.000000,1.000000,1.000000" (Variables|FireWeapon|GetSpread))) "TraceTypeQuery1" false 0 "None"))
    (bind _output_get (Variables|Default|SetHitResuit _outhit_2))
    (return _output_get)
    (else
      (return (Variables|Default|GetHitResuit)))))

(fn TraceEndPoint
  (params (HitResult :type Hit%20Result%20Structure))
  (bind (_bblockinghit _binitialoverlap _time _distance _location _impactpoint _normal _impactnormal _physmat _hitactor _hitcomponent _hitbonename _bonename _hititem _elementindex _faceindex _tracestart _traceend) (Collision|BreakHitResult HitResult))
  (if _bblockinghit
    (Variables|Default|SetEndLineTrace _impactpoint)
    (else
      (Variables|Default|SetEndLineTrace _traceend))))

(fn TraceFX
  (bind _returnvalue (Niagara|SpawnSystematLocation (Variables|Default|GetTraceFXSystem) (Transformation|GetSocketLocation (Variables|Default|GetWeaponMesh) "MuzzleFlash")))
  (Niagara|SetNiagaraVariable(Vector3) _returnvalue "TraceTarget" (Variables|Default|GetEndLineTrace)))

(fn AmmoNotEmpty
  (return (> (Variables|Ammo|GetCurrentAmmo) 0)))

(fn MagazinFull
  (return (== (Variables|Ammo|GetAmmoMagazin) (Variables|Ammo|GetMaxAmmoMagazin))))

(fn CalculateAmmo
  (if (< (Variables|Ammo|GetCurrentAmmo) (- (Variables|Ammo|GetMaxAmmoMagazin) (Variables|Ammo|GetAmmoMagazin)))
    (Variables|Ammo|SetAmmoMagazin (+ (Variables|Ammo|GetAmmoMagazin) (Variables|Ammo|GetCurrentAmmo)))
    (Variables|Ammo|SetCurrentAmmo 0)
    (else
      (bind _output_get (LocalVariables|SetAddMagazinAmmo (- (Variables|Ammo|GetMaxAmmoMagazin) (Variables|Ammo|GetAmmoMagazin))))
      (Variables|Ammo|SetCurrentAmmo (- (Variables|Ammo|GetCurrentAmmo) _output_get))
      (Variables|Ammo|SetAmmoMagazin (+ (Variables|Ammo|GetAmmoMagazin) (LocalVariables|GetAddMagazinAmmo))))))